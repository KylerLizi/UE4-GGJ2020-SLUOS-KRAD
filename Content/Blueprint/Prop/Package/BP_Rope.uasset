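; BP_Rope is a package prop for the rope in Level 1, whose package event advances the dialogue and can trigger the move to Level 2.
; On BeginPlay it caches the first drawer and player found in the world.
; Each package event calls the drawer's SuoHuiQu, then either plays first-time dialogue or later dialogue plus the player's Level 2 load, based on IsFirst.
; Construction assigns M_Light as the outline material.
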(event `self.ReceiveBeginPlay`
  (`parent.ReceiveBeginPlay`)
  (bind _outactors (`GameplayStatics.GetAllActorsOfClass` "/Game/Blueprint/Prop/Interactive/BP_Drawer.BP_Drawer_C"))
  (set `self.Drawer` (`|GetArrayItem` _outactors))
  (bind _outactors_2 (`GameplayStatics.GetAllActorsOfClass` "/Game/Blueprint/Player/BP_Player.BP_Player_C"))
  (set `self.BP_Player` (`|GetArrayItem` _outactors_2)))

(event `self.PackageEvent`
  (`/Game/Blueprint/Prop/Interactive/BP_Drawer.SuoHuiQu` (`self.Drawer`))
  (`parent.PackageEvent`)
  (if (`self.IsFirst`)
    (`/Engine/EditorBlueprintResources/StandardMacros.DoOnce` false
      (:`Completed`
        (`/Game/GameMode/MyHUD.Level 1Dialogue` (`self.BP_HUD`) 4)
        (set `self.IsFirst` false)))
    (else
      (`/Game/GameMode/MyHUD.Level 1Dialogue` (`self.BP_HUD`) 11)
      (`/Game/Blueprint/Player/BP_Player.LoadLevel2` (`self.BP_Player`)))))

(fn `UserConstructionScript`
  (`parent.UserConstructionScript`)
  (set `self.M_Inst_Outline` "/Game/Meshs/Outline/Material/M_Light.M_Light"))