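; BP_Key is a key prop that builds on a parent package-item Blueprint and triggers a Level 1 dialogue line.
; Its PackageEvent override runs the parent logic, then uses DoOnce so the HUD dialogue call fires only the first time.
; The construction script runs the parent's setup and sets the outline material to M_Light.
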(event `self.ReceiveBeginPlay`
  (`parent.ReceiveBeginPlay`))

(event `self.PackageEvent`
  (`parent.PackageEvent`)
  (`/Engine/EditorBlueprintResources/StandardMacros.DoOnce` false
    (:`Completed`
      (`/Game/GameMode/MyHUD.Level 1Dialogue` (`self.BP_HUD`) 5))))

(fn `UserConstructionScript`
  (`parent.UserConstructionScript`)
  (set `self.M_Inst_Outline` "/Game/Meshs/Outline/Material/M_Light.M_Light"))