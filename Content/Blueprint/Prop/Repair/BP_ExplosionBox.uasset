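; A repairable box prop that reassembles from an exploded state and gains the "Move" tag once restored.
; RepairEvent clears the Prop mesh, hides the outline, plays a restore sound and flags the ExplosionMesh Anim Blueprint to reverse the explosion.
; After a timed delay it sets a second animation flag and swaps in the intact static cube.
; A one-shot HUD call then triggers Level 1 dialogue.
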(event `self.RepairEvent`
  (`StaticMeshComponent.SetStaticMesh` (`self.Prop`) null)
  (`self.HideOutline`)
  (bind _asanim_xiangziexplosion (cast `/Game/Animations/blueprints/Anim_xiangziexplosion` (`SkeletalMeshComponent.GetAnimInstance` (`self.ExplosionMesh`))))
  (set `/Game/Animations/blueprints/Anim_xiangziexplosion.isReverseExplode?` true _asanim_xiangziexplosion)
  (`/Game/Audio/Audio.BoxRestore` (`self.BP_Audio`))
  (`KismetSystemLibrary.Delay` 3.2)
  (set `/Game/Animations/blueprints/Anim_xiangziexplosion.isBeforeExplode?` true _asanim_xiangziexplosion)
  (`StaticMeshComponent.SetStaticMesh` (`self.Prop`) "/Game/Animations/Assets/SM_ExplosionCube.SM_ExplosionCube")
  (`KismetArrayLibrary.Array_Add` (`self.Tags`) "Move")
  (`KismetSystemLibrary.Delay` 1.0)
  (`/Engine/EditorBlueprintResources/StandardMacros.DoOnce` false
    (:`Completed`
      (`/Game/GameMode/MyHUD.Level 1Dialogue` (`self.BP_HUD`) 2))))

(fn `UserConstructionScript`
  (`parent.UserConstructionScript`))