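; BP_Box is an interactive chest prop that toggles a rotation of its BaoxiangBaoxiang1 component when used.
; InteractiveEvent drives a FlipFlop that alternately plays and reverses a timeline, setting IsClose true on play and false on reverse.
; Each timeline update scales the track value by BoxRotation to set the component's relative roll, and hides the interaction outline.
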(event `self.InteractiveEvent`
  (`/Engine/EditorBlueprintResources/StandardMacros.FlipFlop`
    (:`A`
      (set `self.IsClose` true)
      (bind (_direction `_新建轨迹_0`) (`Timeline|时间轴_0` :!label _label)
        (:`Update`
          (`SceneComponent.K2_SetRelativeRotation` (`self.baoxiang_baoxiang1`) (`KismetMathLibrary.MakeRotator` (* `_新建轨迹_0` (`self.BoxRotation`))) false false)
          (`self.HideOutline`))))
    (:`B`
      (set `self.IsClose` false)
      (goto _label :!via `Reverse`))))

(fn `UserConstructionScript`
  (`parent.UserConstructionScript`))