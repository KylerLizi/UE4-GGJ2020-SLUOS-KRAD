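; Interactive drawer prop that can shift position and slide along world X with a cupboard sound.
; ImmoveEvent offsets the whole actor along negative X and shows a Level 1 HUD dialogue line only once.
; SuoHuiQu (retract) plays the close sound while a timeline moves the Prop relative to its BeginPlay location, then hides the outline.
; The construction script sets MoveOffset before running the parent's construction.
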(event `self.ReceiveBeginPlay`
  (`parent.ReceiveBeginPlay`)
  (set `self.InitLocation` (`SceneComponent.K2_GetComponentLocation` (`self.Prop`))))

(event `self.ImmoveEvent`
  (`self.K2_AddActorWorldOffset` (-35.0 0.0 0.0))
  (`/Engine/EditorBlueprintResources/StandardMacros.DoOnce` false
    (:`Completed`
      (`/Game/GameMode/MyHUD.Level 1Dialogue` (`self.BP_HUD`) 9))))

(event `SuoHuiQu`
  (`/Game/Audio/Audio.CupboardClose` (`self.BP_Audio`))
  (bind (_direction `_新建轨迹_0`) (`Timeline|时间轴_0`)
    (:`Update`
      (`SceneComponent.K2_SetWorldLocation` (`self.Prop`) (+ (`self.InitLocation`) (`KismetMathLibrary.MakeVector` (* `_新建轨迹_0` (`self.Offset`)))) false false))
    (:`Finished`
      (`self.HideOutline`))))

(fn `UserConstructionScript`
  (set `self.MoveOffset` (-45.0 1.0 155.0))
  (`parent.UserConstructionScript`))