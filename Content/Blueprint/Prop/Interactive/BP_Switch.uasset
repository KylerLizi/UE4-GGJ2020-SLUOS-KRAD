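; BP_Switch is an interactive switch prop that toggles a magic aura effect and the repairable state of all BP_ShuGui actors.
; BeginPlay spawns the aura particle and caches every BP_ShuGui in the level.
; A FlipFlop on InteractiveEvent alternates between destroying the aura while enabling CanRepaire, and respawning it with a magic-circle sound while disabling CanRepaire.
; Lookups for BP_ShuGui_2 and BP_ShuGui_3 are unconnected and never run.
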(event `self.ReceiveBeginPlay`
  (`parent.ReceiveBeginPlay`)
  (bind _returnvalue (`GameplayStatics.SpawnEmitterAtLocation` "/Game/Particles/MoFaZhen/Particles/P_ky_healAura.P_ky_healAura" (`self.SpawnLocation`) (struct) (`self.SpawnScale`) false))
  (set `self.FX_Magic` _returnvalue)
  (bind _outactors (`GameplayStatics.GetAllActorsOfClass` "/Game/Blueprint/Prop/Repair/BP_ShuGui.BP_ShuGui_C"))
  (set `self.BP_ShuGui` _outactors))

(event `self.InteractiveEvent`
  (`/Engine/EditorBlueprintResources/StandardMacros.FlipFlop`
    (:`A`
      (`ActorComponent.K2_DestroyComponent` (`self.FX_Magic`))
      (for _array_element (`self.BP_ShuGui`)
        (set `/Game/Blueprint/Prop/Repair/BP_ShuGui.CanRepaire` true _array_element)))
    (:`B`
      (bind _returnvalue (`GameplayStatics.SpawnEmitterAtLocation` "/Game/Particles/MoFaZhen/Particles/P_ky_healAura.P_ky_healAura" (`self.SpawnLocation`) (struct) (`self.SpawnScale`) false))
      (bind _output_get (set `self.FX_Magic` _returnvalue))
      (`PrimitiveComponent.SetCollisionEnabled` _output_get "NoCollision")
      (`/Game/Audio/Audio.MagicCircle` (`self.BP_Audio`))
      (for _array_element_2 (`self.BP_ShuGui`)
        (set `/Game/Blueprint/Prop/Repair/BP_ShuGui.CanRepaire` false _array_element_2)))))

(fn `UserConstructionScript`
  (`parent.UserConstructionScript`))