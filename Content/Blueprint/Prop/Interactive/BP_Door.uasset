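; BP_Door is an interactive door prop that swings open and closed when its InteractiveEvent fires.
; A FlipFlop alternates between playing and reversing a timeline, whose track scaled by DoorRotation sets the Prop's relative yaw.
; Each timeline update also hides the outline.
; The first time the timeline finishes, a DoOnce triggers a Level 1 dialogue line through the HUD.
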(event `self.InteractiveEvent`
  (`/Engine/EditorBlueprintResources/StandardMacros.FlipFlop`
    (:`A`
      (bind (_direction `_新建轨迹_0`) (`Timeline|时间轴_0` :!label _label)
        (:`Update`
          (`SceneComponent.K2_SetRelativeRotation` (`self.Prop`) (`KismetMathLibrary.MakeRotator` 0.0 0.0 (* `_新建轨迹_0` (`self.DoorRotation`))) false false)
          (`self.HideOutline`))
        (:`Finished`
          (`/Engine/EditorBlueprintResources/StandardMacros.DoOnce` false
            (:`Completed`
              (`/Game/GameMode/MyHUD.Level 1Dialogue` (`self.BP_HUD`) 6))))))
    (:`B`
      (goto _label :!via `Reverse`))))

(fn `UserConstructionScript`
  (`parent.UserConstructionScript`))