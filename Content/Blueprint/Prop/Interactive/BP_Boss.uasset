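; BP_Boss is an interactive boss prop that drives Level 3 dialogue through the HUD and catches fire when interacted with again.
; The first InteractiveEvent clears IsFirst and triggers the opening dialogue line.
; Later interactions apply a fire material to the prop, with a DoOnce limiting the second dialogue line and persistent scaled fire emitter to one trigger.
; The construction script sets a tiny outline scale before calling the parent.
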(event `self.InteractiveEvent`
  (if (`self.IsFirst`)
    (set `self.IsFirst` false)
    (`/Engine/EditorBlueprintResources/StandardMacros.DoOnce` false
      (:`Completed`
        (`/Game/GameMode/MyHUD.Level 3Dialogue` (`self.BP_HUD`) 1)))
    (else
      (`PrimitiveComponent.SetMaterial` (`self.Prop`) 0 (`self.FireMaterial`))
      (`/Engine/EditorBlueprintResources/StandardMacros.DoOnce` false
        (:`Completed`
          (`/Game/GameMode/MyHUD.Level 3Dialogue` (`self.BP_HUD`) 2)
          (`GameplayStatics.SpawnEmitterAtLocation` "/Game/Particles/Fire/Particles/Fire/Fire_03.Fire_03" (`self.K2_GetActorLocation`) (struct) (* (`self.VFXScale`) 1.5) false))))))

(fn `UserConstructionScript`
  (set `self.OutlineScale` 0.001)
  (`parent.UserConstructionScript`))