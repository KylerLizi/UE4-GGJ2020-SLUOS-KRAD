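; Base actor for interactable props, with empty Interactive, Repair, Broke, Immove and Dialogue events as hooks.
; It caches the HUD and Audio actors on BeginPlay, and PackageEvent adds its PropAsset to the HUD's package view before destroying the actor.
; Cursor hover spawns a duplicate static mesh with a dynamic outline material set by color and scale, then destroys it when the cursor leaves.
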(event `self.ReceiveBeginPlay`
  (bind _outactors (`GameplayStatics.GetAllActorsOfClass` "/Game/GameMode/MyHUD.MyHUD_C"))
  (set `self.BP_HUD` (`|GetArrayItem` _outactors))
  (bind _outactors_2 (`GameplayStatics.GetAllActorsOfClass` "/Game/Audio/Audio.Audio_C"))
  (set `self.BP_Audio` (`|GetArrayItem` _outactors_2)))

(event `PackageEvent`
  (`/Game/UMG/UMG_package.UpdateView` (cast `/Game/UMG/UMG_package` (`/Game/GameMode/MyHUD.UMG_Package` (`self.BP_HUD`)) :!pure true) (`self.PropAsset`) true)
  (`self.K2_DestroyActor`))

(event `InteractiveEvent`)

(event `RepairEvent`)

(event `BrokeEvent`)

(event `ImmoveEvent`)

(event `DialogueEvent`)

(event `self.ReceiveActorBeginCursorOver`
  (`self.ShowOutline`))

(event `self.ReceiveActorEndCursorOver`
  (`self.HideOutline`))

(fn `HideOutline`
  (if (`self.HasOutline`)
    (`ActorComponent.K2_DestroyComponent` (`self.OutlineMesh`))
    (set `self.HasOutline` false)))

(fn `ShowOutline`
  (if (not (`self.HasOutline`))
    (bind _returnvalue (`AddComponent|NODE_AddStaticMeshComponent-1` :`bManualAttachment` true :`RelativeTransform` (`SceneComponent.K2_GetComponentToWorld` (`self.Prop`))))
    (bind _output_get (set `self.OutlineMesh` _returnvalue))
    (`StaticMeshComponent.SetStaticMesh` _output_get (`StaticMeshComponent.StaticMesh` (`self.Prop`)))
    (bind _returnvalue_2 (`PrimitiveComponent.CreateDynamicMaterialInstance` (`self.OutlineMesh`) 0 (`self.M_Inst_Outline`) "None"))
    (`MaterialInstanceDynamic.SetVectorParameterValue` _returnvalue_2 "Color" (`self.OutlineColor`))
    (`MaterialInstanceDynamic.SetScalarParameterValue` _returnvalue_2 "Scale" (`self.OutlineScale`))
    (set `self.HasOutline` true)))

(fn `UserConstructionScript`)