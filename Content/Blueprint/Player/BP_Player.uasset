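; Player Blueprint for a point-and-click puzzle level, handling mouse interaction with props, inventory and horizontal camera movement.
; Cursor traces find BP_PropParent actors, whose tags route clicks to interact, dialogue, break, repair, pickup or bag events.
; Carried props follow the cursor each Tick with collision off and trace-ignored until placed on an Immove target.
; Items spawned from the E-toggled bag enter carry mode and leave the inventory UI when placed.
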(event `self.ReceiveBeginPlay`
  (bind _outactors (`GameplayStatics.GetAllActorsOfClass` "/Game/GameMode/MyHUD.MyHUD_C"))
  (set `self.BP_HUD` (`|GetArrayItem` _outactors))
  (bind _outactors_2 (`GameplayStatics.GetAllActorsOfClass` "/Game/Audio/Audio.Audio_C"))
  (bind _output_get (set `self.BP_Audio` (`|GetArrayItem` _outactors_2)))
  (`/Game/Audio/Audio.OpenBGM` _output_get))

(event `self.ReceiveTick`
  (params (DeltaSeconds :type "Float (single-precision)"))
  (`self.Moving`))

(event `Key|LeftMouseButton`
  (params (Key :type "Key Structure"))
  ;[1 0.4301 0.4879] 物品交互
  (:`Pressed`
    (bind _success (`self.LineTrace`))
    (if _success
      (`|ExecutionSequence`
        (:`then_0`
          (bind (_exist _prop) (`self.ExistTag`))
          (if _exist
            (for _array_element (`Actor.Tags` (`self.HitActor`))
              (switch `string` (`KismetStringLibrary.Conv_NameToString` _array_element)
                (:`Interactive`
                  (`/Game/Blueprint/Prop/BP_PropParent.InteractiveEvent` _prop)
                  (`/Game/Blueprint/Prop/BP_PropParent.DialogueEvent` _prop))
                (:`Move`
                  (`self.PullUp`))
                (:`Immove`
                  (`self.PullDown`)
                  (`/Game/Blueprint/Prop/BP_PropParent.DialogueEvent` _prop))))))
        (:`then_1`
          ;;[1 1 1] 会销毁 不能用Foreachloop 会报错
          (if (`self.ActorHasTag` (`self.HitActor`) (`self.PackageTag`))
            (`/Game/Blueprint/Prop/BP_PropParent.DialogueEvent` _prop)
            (`/Game/Blueprint/Prop/BP_PropParent.PackageEvent` _prop)))))))

(event `PackageSpawn`
  ;[1 1 1] 从背包拿出来就实例化一个物品
  (set `self.Spawing` true)
  (bind _returnvalue (`|SpawnActorFromClass` (`self.SpawnClass`) (`KismetMathLibrary.MakeTransform` (0.0 0.0 0.0)) "Undefined" "OverrideRootScale" null null))
  (bind _output_get (set `self.HitActor` _returnvalue))
  (`self.PullUp`)
  (`/Engine/EditorBlueprintResources/StandardMacros.DoOnce` false
    (:`Completed`
      (`/Game/GameMode/MyHUD.Level 1Dialogue` (`self.BP_HUD`) 8)
      (bind (_asbp_rope _bsuccess) (cast `/Game/Blueprint/Prop/Package/BP_Rope` _output_get :!pure true))
      (if _bsuccess
        (set `/Game/Blueprint/Prop/Package/BP_Rope.IsFirst` false _asbp_rope)))))

(event `Key|RightMouseButton`
  (params (Key :type "Key Structure"))
  ;[1 0.4301 0.4879] 物品交互
  (:`Pressed`
    (bind _success (`self.LineTrace`))
    (if _success
      (bind (_exist _prop) (`self.ExistTag`))
      (if _exist
        (for _array_element (`Actor.Tags` (`self.HitActor`))
          (switch `string` (`KismetStringLibrary.Conv_NameToString` _array_element)
            (:`Broke`
              (`/Game/Blueprint/Prop/BP_PropParent.BrokeEvent` _prop)
              (`/Game/Blueprint/Prop/BP_PropParent.DialogueEvent` _prop))
            (:`Repair`
              (`/Game/Blueprint/Prop/BP_PropParent.RepairEvent` _prop)
              (`/Game/Blueprint/Prop/BP_PropParent.DialogueEvent` _prop))))))))

(event `Key|E`
  (params (Key :type "Key Structure"))
  (bind _umg_package (`/Game/GameMode/MyHUD.UMG_Package` (`self.BP_HUD`)))
  ;[1 1 1] 背包
  (:`Pressed`
    (`/Engine/EditorBlueprintResources/StandardMacros.FlipFlop`
      (:`A`
        (`|ExecutionSequence`
          (:`then_0`
            (`/Engine/EditorBlueprintResources/StandardMacros.DoOnce` false
              (:`Completed`
                (`/Game/GameMode/MyHUD.Level 1Dialogue` (`self.BP_HUD`) 7)
                (`KismetSystemLibrary.Delay` 3.0))))
          (:`then_1`
            (`/Game/Audio/Audio.Bag` (`self.BP_Audio`))
            (`Widget.SetVisibility` _umg_package "Visible"))))
      (:`B`
        (`Widget.SetVisibility` _umg_package "Hidden")))))

(event `InputAction|GoOn`
  (params (Key :type "Key Structure"))
  (:`Pressed`
    (`/Game/GameMode/MyHUD.EndDialogue` (`self.BP_HUD`))))

(event `Key|SpaceBar`
  (params (Key :type "Key Structure"))
  (:`Pressed`
    (`/Game/UMG/end.SkipEnd` (`/Game/GameMode/MyHUD.End` (`self.BP_HUD`)))))

(event `InputAxis|LeftMove`
  (params (AxisValue :type "Float (single-precision)"))
  (`self.K2_AddActorWorldOffset` (`KismetMathLibrary.MakeVector` (* AxisValue 3.0))))

(event `InputAxis|RightMove`
  (params (AxisValue :type "Float (single-precision)"))
  (`self.K2_AddActorWorldOffset` (`KismetMathLibrary.MakeVector` (* AxisValue 3.0))))

(event `Key|Q`
  (params (Key :type "Key Structure"))
  (:`Pressed`
    (`self.K2_SetActorLocation` (`self.1-2`) :!label _label)))

(event `LoadLevel2`
  (goto _label))

(fn `ExistTag`
  (returns (Exist :type Boolean) (Prop :type "/Game/Blueprint/Prop/BP_PropParent Object Reference"))
  (bind _asbp_prop_parent (cast `/Game/Blueprint/Prop/BP_PropParent` (`self.HitActor`)))
  (return (> (`KismetArrayLibrary.Array_Length` (`Actor.Tags` (`self.HitActor`))) 0) _asbp_prop_parent))

(fn `LineTrace`
  (returns (Success :type Boolean))
  (bind (_worldlocation _worlddirection) (`PlayerController.DeprojectMousePositionToWorld` (`GameplayStatics.GetPlayerController` 0)))
  (bind (_outhit _returnvalue) (`KismetSystemLibrary.LineTraceSingle` _worldlocation (+ _worldlocation (* _worlddirection 100000.0)) "TraceTypeQuery1" true (`self.IgnoreTrace`)))
  (bind (_bblockinghit _binitialoverlap _time _distance _location _impactpoint _normal _impactnormal _physmat _hitactor) (`GameplayStatics.BreakHitResult` _outhit))
  (set `self.HitLocation` _location)
  (bind _asbp_prop_parent (cast `/Game/Blueprint/Prop/BP_PropParent` _hitactor))
  (set `self.HitActor` _asbp_prop_parent)
  (return _returnvalue))

(fn `Moving`
  (bind _moveactor (`self.MoveActor`))
  ;[1 0.2812 0] 跟随鼠标位置移动
  (if (== (`self.MoveTag`) (`self.CurrentTag`))
    (`self.K2_SetActorLocation` _moveactor (`.Location` (`GameplayStatics.BreakHitResult` (`PlayerController.GetHitResultUnderCursorByChannel` (`GameplayStatics.GetPlayerController` 0) "TraceTypeQuery1" true))) false false)
    (`/Game/Blueprint/Prop/BP_PropParent.HideOutline` (cast `/Game/Blueprint/Prop/BP_PropParent` _moveactor :!pure true))))

(fn `PullDown`
  (bind _hitactor (`self.HitActor`))
  (bind (_asbp_prop_parent _bsuccess) (cast `/Game/Blueprint/Prop/BP_PropParent` _hitactor :!pure true))
  ;[0 1 0.3906] 放置物体
  (set `self.CurrentTag` (`self.ImmoveTag`))
  (if (and (> (`KismetArrayLibrary.Array_Length` (`self.IgnoreTrace`)) 0) _bsuccess)
    (`self.K2_SetActorLocation` (`self.MoveActor`) (`KismetMathLibrary.SelectVector` (`self.HitLocation`) (+ (`/Game/Blueprint/Prop/BP_PropParent.MoveOffset` _asbp_prop_parent) (`self.K2_GetActorLocation` _hitactor)) (`.bSuccess` (cast `/Game/Blueprint/Prop/Repair/BP_ExplosionBox` (`self.MoveActor`) :!pure true))) false false)
    (`KismetArrayLibrary.Array_Clear` (`self.IgnoreTrace`))
    (`self.SetActorEnableCollision` (`self.MoveActor`) true)
    (if (`.bSuccess` (cast `/Game/Blueprint/Prop/Package/BP_Key` (`self.MoveActor`) :!pure true))
      (`self.SetActorHiddenInGame` (`self.MoveActor`) true)
      (`/Game/GameMode/MyHUD.Level 1Dialogue` (`self.BP_HUD`) 10)
      (else
        (`/Game/Blueprint/Prop/BP_PropParent.ImmoveEvent` (cast `/Game/Blueprint/Prop/BP_PropParent` (`self.HitActor`) :!pure true))))
    ;[1 1 1] 从背包中实例化出来的
    (if (`self.Spawing`)
      (`/Game/UMG/UMG_package.UpdateView` (cast `/Game/UMG/UMG_package` (`/Game/GameMode/MyHUD.UMG_Package` (`self.BP_HUD`)) :!pure true) (`/Game/Blueprint/Prop/BP_PropParent.PropAsset` (cast `/Game/Blueprint/Prop/BP_PropParent` (`self.MoveActor`) :!pure true)) false)
      (set `self.Spawing` false))))

(fn `PullUp`
  (bind _hitactor (`self.HitActor`))
  (set `self.CurrentTag` (`self.MoveTag`))
  ;[1 1 1] 忽略正在移动物体的射线检测
  (`KismetArrayLibrary.Array_AddUnique` (`self.IgnoreTrace`) _hitactor)
  (set `self.MoveActor` _hitactor)
  (`self.SetActorEnableCollision` _hitactor false))

(fn `UserConstructionScript`)