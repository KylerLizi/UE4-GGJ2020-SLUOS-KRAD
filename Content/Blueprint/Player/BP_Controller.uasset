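; BP_Controller is an unfinished controller Blueprint for AI patrol (xunluo) movement between target points.
; The xunluo event calls the empty AIArrivedTarget function, then issues AIMoveTo when Targetpoint differs from Currentpoint, updating Currentpoint first.
; Logic that gathers all TargetPoint actors and starts a one-shot timer for xunluo is disconnected, and BeginPlay is empty, so nothing here starts the patrol.
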(event `self.ReceiveBeginPlay`)

(event `xunluo`
  (`self.AI Arrived Target`)
  (if (!= (`self.targetpoint`) (`self.currentpoint`))
    (set `self.currentpoint` (`self.targetpoint`))
    (`|AIMoveTo` null (0.0 0.0 0.0) (`self.currentpoint`))))

(fn `AI Arrived Target`)

(fn `UserConstructionScript`)